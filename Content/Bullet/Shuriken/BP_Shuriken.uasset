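; BP_Shuriken is a pooled 2D shuriken projectile that damages enemies it overlaps and keeps flying after hits.
; SetBulletValue configures flipbook, velocity, scale, damage, target and color, then starts a lifetime timer.
; Sphere overlaps track struck enemies, sending damage with impact force on first contact and a separate damage-only message on repeats.
; When the timer ends, it clears its sprite and hit list, moves far away and switches state for reuse instead of being destroyed.
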(event `self.Sphere.OnComponentBeginOverlap`
  (params (OverlappedComponent :type "PrimitiveComponent Object Reference") (OtherActor :type "Actor Object Reference") (OtherComp :type "PrimitiveComponent Object Reference") (OtherBodyIndex :type Integer) (bFromSweep :type Boolean) (SweepResult :type "HitResult Structure (by ref)"))
  (switch `name` (`self.Bullet Target`)
    (:`enemy`
      (if (`KismetArrayLibrary.Array_Contains` (`self.EnemyAttack`) OtherActor)
        (message `/Game/Interface/BP_Interface_Player.BeingAttack` OtherActor (`self.Bullet Damage`) self)
        (else
          (`KismetArrayLibrary.Array_AddUnique` (`self.EnemyAttack`))
          (message `/Game/Interface/BP_Interface_Enemy.Being Attacked` OtherActor (`self.Bullet Damage`) (`self.Impact Force`)))))))

(fn `BulletObejectRecycling`
  (`PaperFlipbookComponent.SetFlipbook` (`self.PaperFlipbook`) null)
  (`self.K2_SetActorLocation` (10000.0 10000.0 -1000.0))
  (set `self.BulletState` "NewEnumerator1")
  (`KismetArrayLibrary.Array_Clear` (`self.EnemyAttack`)))

(fn `setBulletValue`
  (params (BulletPic :type "PaperFlipbook Object Reference") (BulletDamage :type "Float (double-precision)") (BulletSpeed :type "Vector Structure") (BulletSize :type "Vector Structure") (BulletTargetSize :type "Vector Structure") (BulletTarget :type Name) (LifeCycle :type "Float (double-precision)") (ImpactForce :type "Float (double-precision)") (Color :type "LinearColor Structure"))
  (`PaperFlipbookComponent.SetFlipbook` (`self.PaperFlipbook`) BulletPic)
  (set `self.Bullet Damage` BulletDamage)
  (set `MovementComponent.Velocity` BulletSpeed (`self.ProjectileMovement`))
  (`SceneComponent.SetWorldScale3D` (`self.PaperFlipbook`) BulletSize)
  (`SceneComponent.SetWorldScale3D` (`self.Sphere`) BulletTargetSize)
  (set `self.Bullet Target` BulletTarget)
  (set `self.BulletState` "NewEnumerator0")
  (set `self.Impact Force` (`local.ImpactForce`))
  (`PaperFlipbookComponent.SetSpriteColor` (`self.PaperFlipbook`) Color)
  (`KismetSystemLibrary.K2_SetTimer` null "BulletObejectRecycling" LifeCycle))

(fn `UserConstructionScript`)