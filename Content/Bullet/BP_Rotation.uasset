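; BP_Rotation is a bullet actor that forms a rotating ring of BP_IceSword actors around itself.
; SetValue stores spin rate, radius, count and sword properties; BeginToRotation destroys existing swords, applies the rate to RotatingMovement and spawns new ones evenly via sine and cosine.
; Each sword receives its properties and attaches to the root so the ring spins together.
; BeginPlay is empty, and the event graph's BeginToRotation call is disconnected.
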(event `self.ReceiveBeginPlay`)

(fn `BeginToRotation`
  (bind (_returnvalue_x _returnvalue_y _returnvalue_z) (`KismetMathLibrary.BreakVector` (`self.K2_GetActorLocation`)))
  (bind _itemnum (`self.ItemNum`))
  (bind _iceswordarry (`self.IceSwordArry`))
  (if (not (`KismetArrayLibrary.Array_IsEmpty` _iceswordarry))
    (for _array_element _iceswordarry
      (`/Engine/EditorBlueprintResources/StandardMacros.IsValid` _array_element
        (:`Is Valid`
          (`self.K2_DestroyActor` _array_element)))))
  (set `RotatingMovementComponent.RotationRate` (`self.旋转速率`) (`self.RotatingMovement`))
  (set `self.Angle` (/ (* (`KismetMathLibrary.GetPI`) 2.0) _itemnum))
  (for _index (range _itemnum)
    (bind _returnvalue (* (`self.Angle`) _index))
    (bind _returnvalue_2 (`|SpawnActorFromClass` "/Game/Bullet/IceSword/BP_IceSword.BP_IceSword_C" (`KismetMathLibrary.MakeTransform` (`KismetMathLibrary.MakeVector` (+ (* (`KismetMathLibrary.Cos` _returnvalue) (`self.R`)) _returnvalue_x) (+ (* (`KismetMathLibrary.Sin` _returnvalue) (`self.R`)) _returnvalue_y) _returnvalue_z)) "AlwaysSpawn" "OverrideRootScale" null null))
    (`KismetArrayLibrary.Array_AddUnique` (`self.IceSwordArry`) _returnvalue_2)
    (`/Game/Bullet/IceSword/BP_IceSword.setIceSwordValue` _returnvalue_2 (`self.Bullet Pic`) (`self.Damage`) (`self.Bullet Size`) (`self.Impact Force`) (`self.Color`))
    (`self.K2_AttachToComponent` _returnvalue_2 (`self.DefaultSceneRoot`) "None" "KeepWorld" "KeepRelative" "KeepRelative" true)))

(fn `setValue`
  (params (`旋转速率` :type "Rotator Structure") (R :type "Float (double-precision)") (ItemNum :type Integer) (`Bullet Pic` :type "PaperFlipbook Object Reference") (Damage :type "Float (double-precision)") (`Bullet Size` :type "Vector Structure") (`Impact Force` :type "Float (double-precision)") (Color :type "LinearColor Structure"))
  (set `self.旋转速率` `旋转速率`)
  (set `self.R` R)
  (set `self.ItemNum` ItemNum)
  (set `self.Bullet Pic` `Bullet Pic`)
  (set `self.Damage` Damage)
  (set `self.Bullet Size` `Bullet Size`)
  (set `self.Impact Force` `Impact Force`)
  (set `self.Color` Color))

(fn `UserConstructionScript`)