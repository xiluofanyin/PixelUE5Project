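; BP_IceSword is the ice sword bullet, a Paper2D flipbook with a sphere hitbox that damages enemies it touches.
; On sphere overlap with an actor tagged "enemy", it sends BeingAttackedMessage with the player's damage plus its own, along with an impact force.
; SetIceSwordValue configures the flipbook, tint, damage, impact force and a shared scale for sprite and sphere.
; It contains no movement or destroy-on-hit logic.
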(event `self.Sphere.OnComponentBeginOverlap`
  (params (OverlappedComponent :type "PrimitiveComponent Object Reference") (OtherActor :type "Actor Object Reference") (OtherComp :type "PrimitiveComponent Object Reference") (OtherBodyIndex :type Integer) (bFromSweep :type Boolean) (SweepResult :type "HitResult Structure (by ref)"))
  (if (`self.ActorHasTag` OtherActor "enemy")
    (message `/Game/Interface/BP_Interface_Enemy.Being Attacked` OtherActor (+ (`/Game/BluePrints/BP_Player.Damage` (`/Game/BluePrints/Instance/BL_PublicBPLibrary.GetPlayer`)) (`self.Damage`)) (`self.Impact Force`))))

(fn `setIceSwordValue`
  (params (BulletPic :type "PaperFlipbook Object Reference") (Damage :type "Float (double-precision)") (BulletSize :type "Vector Structure") (ImpactForce :type "Float (double-precision)") (Color :type "LinearColor Structure"))
  (`PaperFlipbookComponent.SetFlipbook` (`self.PaperFlipbook`) BulletPic)
  (set `self.Damage` Damage)
  (`SceneComponent.SetWorldScale3D` (`self.PaperFlipbook`) BulletSize)
  (`SceneComponent.SetWorldScale3D` (`self.Sphere`) BulletSize)
  (set `self.Impact Force` (`local.ImpactForce`))
  (`PaperFlipbookComponent.SetSpriteColor` (`self.PaperFlipbook`) Color))

(fn `UserConstructionScript`)