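; Base pooled 2D sprite enemy that chases the player, takes hits and recycles on death, configured from the DAEnemy data.
; A looping timer teleports it to an off-screen navmesh point near the player, then starts a repeating AI MoveTo chase.
; Hits flash red, show damage numbers and apply mass-scaled knockback.
; At zero HP it disables itself, leaves the active pool, parks below the map and asks ObjectPooling for more enemies.
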(event `self.ReceiveBeginPlay`
  (bind _da_enemy (`self.DA_Enemy`))
  ;[1 1 1] Constructor
  (bind _asabp_enemies (cast `/Game/Enemies/ABP_Enemies` (`self.GetAnimInstance`)))
  (bind _output_get (set `self.As ABP Enemies` _asabp_enemies))
  (set `/Game/Enemies/ABP_Enemies.EnemyAni` (`self.Enemy Ani`) _output_get)
  (set `self.Enemy Ani` (`/Game/DataAsset/Enemy/DA_Enemy.Enemy_Ani` _da_enemy))
  (set `CharacterMovementComponent.MaxWalkSpeed` (`/Game/DataAsset/Enemy/DA_Enemy.Enemy_Speed` _da_enemy) (`self.CharacterMovement`))
  (set `self.Enemy Mass` (`/Game/DataAsset/Enemy/DA_Enemy.Enemy_Mass` _da_enemy))
  (set `self.Enemy HP` (`/Game/DataAsset/Enemy/DA_Enemy.Enemy_HP` _da_enemy))
  (`KismetSystemLibrary.K2_SetTimer` null "SetEnemyBirthPosition" 0.3 true))

(event `BeginMoving`
  (bind _returnvalue (`GameplayStatics.GetPlayerPawn` 0))
  ;[1 1 1] Attack
  (`KismetSystemLibrary.Delay` 0.2)
  (`/Engine/EditorBlueprintResources/StandardMacros.IsValid` _returnvalue
    (:`Is Valid`
      (`CharacterMovementComponent.SetMovementMode` (`self.CharacterMovement`) "MOVE_Walking" 0)
      (`|AIMoveTo` self (0.0 0.0 0.0) _returnvalue
        (:`OnSuccess`
          (`KismetSystemLibrary.K2_ClearAndInvalidateTimerHandle` (`self.FindWayTimer`))
          (`self.BeginMoving`))
        (:`OnFail`
          (bind _returnvalue_2 (`KismetSystemLibrary.K2_SetTimerDelegate` (`|CreateDelegate` :!event `BeginMoving`) 0.5))
          (set `self.FindWayTimer` _returnvalue_2))))))

(event `self.ReceiveTick`
  (params (DeltaSeconds :type "Float (single-precision)"))
  (`self.K2_SetActorRotation` (struct)))

(event `/Game/Interface/BP_Interface_Enemy.Being Attacked`
  (params (AttackeDamage :type "Float (double-precision)") (ImpactForce :type "Float (double-precision)"))
  ;[1 1 1] BeingAttack
  (`PaperFlipbookComponent.SetSpriteColor` (`self.Sprite`) (struct :`R` 1.0 :`A` 1.0))
  (`self.BeingAttackNumDisplay` (`KismetTextLibrary.Conv_IntToText` (`KismetMathLibrary.FTrunc` AttackeDamage)))
  (`GameplayStatics.PlaySound2D` "/Game/Sound/SoundEffect/Attack_Sound.Attack_Sound" 1.0 1.0 0.0 null null)
  (`self.Replused` ImpactForce)
  (bind _returnvalue (`self.EnemyHPCalculate` AttackeDamage))
  (if _returnvalue
    (`self.DeathRecycling`)
    (else
      (`KismetSystemLibrary.Delay` 0.1)
      (`PaperFlipbookComponent.SetSpriteColor` (`self.Sprite`) (struct :`R` 1.0 :`G` 1.0 :`B` 1.0 :`A` 1.0)))))

(event `Replused`
  (params (ImpactForce :type "Float (double-precision)"))
  ;[1 1 1] Replused
  (`MovementComponent.StopMovementImmediately` (`self.CharacterMovement`))
  (`self.LaunchCharacter` (* (/ ImpactForce (`self.Enemy Mass`)) (`KismetMathLibrary.GetDirectionUnitVector` (`self.K2_GetActorLocation` (`GameplayStatics.GetPlayerPawn` 0)) (`self.K2_GetActorLocation`))) true))

(fn `BeingAttackNumDisplay`
  (params (DamageNum :type Text))
  (`self.DamageContrainer`
    (:`then`
      _)
    (:`else`
      (bind _returnvalue (`|SpawnActorFromClass` "/Game/UI/BP_DamageContrainer.BP_DamageContrainer_C" (`KismetMathLibrary.MakeTransform` (`SceneComponent.K2_GetComponentLocation` (`self.Sprite`))) "Undefined" "OverrideRootScale" null null))
      (set `self.DamageContrainer` _returnvalue)
      (`self.K2_AttachToComponent` (`self.DamageContrainer`) (`self.Sprite`) "None" "KeepWorld" "KeepWorld" "KeepWorld" true)))
  (`/Game/UI/BP_DamageContrainer.DisplayDamage` (`self.DamageContrainer`) DamageNum))

(fn `DeathRecycling`
  (`self.SetActorTickEnabled` false)
  (`ActorComponent.SetComponentTickEnabled` (`self.AnimationComponent`) false)
  (`CharacterMovementComponent.SetMovementMode` (`self.CharacterMovement`) "MOVE_None" 0)
  (set `self.isDeath` true)
  (`PrimitiveComponent.SetCollisionResponseToChannel` (`self.CapsuleComponent`) "ECC_Pawn" "ECR_Ignore")
  (`KismetSystemLibrary.K2_ClearAndInvalidateTimerHandle` (`self.FindWayTimer`))
  (bind _returnvalue (`KismetArrayLibrary.Array_RemoveItem` (`/Game/BluePrints/BP_ObjectPooling.DynamicEnemyPooling` (`/Game/BluePrints/Instance/GI_Instance_Bullet.ObjectPooling` (`/Game/BluePrints/Instance/BL_PublicBPLibrary.GetGameInstance`))) self))
  (if _returnvalue
    (bind _returnvalue_2 (`self.K2_TeleportTo` (0.0 0.0 -1000.0)))
    (if _returnvalue_2
      (`PaperFlipbookComponent.SetSpriteColor` (`self.Sprite`) (struct :`R` 1.0 :`G` 1.0 :`B` 1.0 :`A` 1.0))
      (`/Game/UI/BP_DamageContrainer.RemoveDamage` (`self.DamageContrainer`))
      (`/Game/BluePrints/BP_ObjectPooling.setMoreEnemy` (`/Game/BluePrints/Instance/GI_Instance_Bullet.ObjectPooling` (`/Game/BluePrints/Instance/BL_PublicBPLibrary.GetGameInstance`))))))

(fn `EnemyHPCalculate`
  (params (Damage :type "Float (double-precision)"))
  (returns (ReturnValue :type Boolean))
  (bind _output_get (set `self.Enemy HP` (`KismetMathLibrary.FClamp` (- (`self.Enemy HP`) Damage) 0.0 (`self.Enemy HP`))))
  (return (== _output_get 0.0)))

(fn `SetEnemyBirthPosition`
  (locals (RandomPosition :type "Vector Structure" :default (0.0 0.0 0.0)))
  (bind _randomlocation (`NavigationSystemV1.K2_GetRandomLocationInNavigableRadius` (`self.K2_GetActorLocation` (`GameplayStatics.GetPlayerPawn` 0)) 900.0 null null))
  (set `local.RandomPosition` _randomlocation)
  (if (not (`/Game/BluePrints/Instance/BL_PublicBPLibrary.CheckisInPlayerScreen` (`local.RandomPosition`)))
    (bind _returnvalue (`self.K2_TeleportTo` (+ (`local.RandomPosition`) (0.0 0.0 15.0))))
    (if _returnvalue
      (`KismetSystemLibrary.K2_ClearTimer` null "SetEnemyBirthPosition")
      (`self.SetActorTickEnabled` true)
      (`ActorComponent.SetComponentTickEnabled` (`self.AnimationComponent`) true)
      (set `self.isDeath` false)
      (`PrimitiveComponent.SetCollisionResponseToChannel` (`self.CapsuleComponent`) "ECC_Pawn" "ECR_Overlap")
      (`self.BeginMoving`))))

(fn `UserConstructionScript`)