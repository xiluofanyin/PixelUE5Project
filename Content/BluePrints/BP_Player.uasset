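; Player character for a sprite-based auto-attack action game, handling movement, health, pickups, EXP leveling and game over.
; Base stats come from PlayerDA; level-ups open the skill UI, and learned skills apply passive boosts or tiered weapon upgrades seeded from DT_SkillTable.
; Cursor-aimed Shuriken fires on input, Thunder strikes randomly nearby on a looping timer, and Ice Sword uses an attached BP_Rotation.
; Shuriken and Thunder draw bullets from the GameInstance's object pool.
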(event `self.ReceiveBeginPlay`
  (bind _asgi_instance_bullet (`/Game/BluePrints/Instance/BL_PublicBPLibrary.GetGameInstance`))
  (set `/Game/BluePrints/Instance/GI_Instance_Bullet.Player` self _asgi_instance_bullet)
  (set `self.As GI Instance Bullet` _asgi_instance_bullet)
  (`self.PlayerDAInit`)
  (`self.HUDInit`)
  (`self.PositiveSkillUpgrade` (`self.Start Skill Tag`))
  (bind _returnvalue (`GameplayStatics.CreateSound2D` (`|GetArrayItem` (`self.Sound`) (`self.IndexOfBGM`)) 1.0 1.0 0.0 null))
  (bind _output_get (set `self.BGM` _returnvalue))
  (`AudioComponent.FadeIn` _output_get 0.0 1.0 0.0 "Linear"))

(event `EnhancedInput|/Game/EnhanceInput/IA_Move`
  (params (ActionValue :type "Vector2D Structure") (ElapsedSeconds :type "Float (double-precision)") (TriggeredSeconds :type "Float (double-precision)") (InputAction :type "InputAction Object Reference" :default "/Game/EnhanceInput/IA_Move.IA_Move"))
  (bind (_x _y) (`KismetMathLibrary.BreakVector2D` ActionValue))
  (:`Triggered`
    (set `self.X` _x)
    (set `self.Y` _y)
    (`self.AddMovementInput` (1.0 0.0 0.0) (`self.X`))
    (`self.AddMovementInput` (0.0 1.0 0.0) (`self.Y`))))

(event `EnhancedInput|/Game/EnhanceInput/IA_Attack`
  (params (ActionValue :type Boolean) (ElapsedSeconds :type "Float (double-precision)") (TriggeredSeconds :type "Float (double-precision)") (InputAction :type "InputAction Object Reference" :default "/Game/EnhanceInput/IA_Attack.IA_Attack"))
  (:`Started`
    (`self.Skill_Shuriken`)))

(event `EnhancedInput|/Game/EnhanceInput/IA_Pause`
  (params (ActionValue :type Boolean) (ElapsedSeconds :type "Float (double-precision)") (TriggeredSeconds :type "Float (double-precision)") (InputAction :type "InputAction Object Reference" :default "/Game/EnhanceInput/IA_Pause.IA_Pause"))
  (:`Triggered`
    (`GameplayStatics.SetGlobalTimeDilation` 0.0)))

(event `/Game/Interface/BP_Interface_Player.GetPickItem`
  (params (Item :type "/Game/Item/BP_BaseItem Object Reference"))
  (set `self.Item` Item)
  (switch `/Game/BluePrints/Enum/Enum_ItemType` (`/Game/Item/BP_BaseItem.Type` Item)
    (:`NewEnumerator0`
      (`self.EXP_Up` (`/Game/Item/BP_BaseItem.EXP Num` (`self.Item`)))
      (`/Engine/EditorBlueprintResources/StandardMacros.IncrementInt` (`self.EXPGetNum`)))
    (:`NewEnumerator1`
      (set `self.CurrentHP` (`KismetMathLibrary.FClamp` (+ (`self.CurrentHP`) 5.0) 0.0 (`self.Max Hp`)))
      (`self.UpdateHPHUD`))
    (:`NewEnumerator2`
      (`SphereComponent.SetSphereRadius` (`self.PickScale`) (`self.OctopusPickScale`) true)
      (`KismetSystemLibrary.Delay` 2.0)
      (`SphereComponent.SetSphereRadius` (`self.PickScale`) (`self.PlayerPickScale`) true))
    (:`NewEnumerator3`
      (`|SpawnActorFromClass` "/Game/Item/BP_KillAll.BP_KillAll_C" (`KismetMathLibrary.MakeTransform` (`self.K2_GetActorLocation`)) "Undefined" "OverrideRootScale" null null))))

(event `/Game/Interface/BP_Interface_Player.BeingAttack`
  (params (Damage :type "Float (double-precision)") (Attacker :type "Actor Object Reference"))
  (`self.PlayerHPCaculate` Damage)
  (`self.BeingAttackedDisplay`))

(event `BeingAttackedDisplay`
  (`PaperFlipbookComponent.SetSpriteColor` (`self.Sprite`) (struct :`R` 1.0 :`B` 0.024837 :`A` 1.0))
  (`KismetSystemLibrary.Delay` 0.1)
  (`PaperFlipbookComponent.SetSpriteColor` (`self.Sprite`) (struct :`R` 1.0 :`G` 1.0 :`B` 1.0 :`A` 1.0)))

(fn `AutoAttack`
  (params (SkillTag :type String))
  (switch `string` SkillTag
    (:`Thunder`
      (`KismetSystemLibrary.K2_SetTimer` null "Skill_Thunder" (`self.ThunderRate`) true))
    (:`IceSword`
      (bind _returnvalue (`|SpawnActorFromClass` "/Game/Bullet/BP_Rotation.BP_Rotation_C" (`KismetMathLibrary.MakeTransform` (`self.K2_GetActorLocation`)) "Undefined" "OverrideRootScale" null null))
      (bind _output_get (set `self.Rotation` _returnvalue))
      (`self.K2_AttachToActor` _output_get self "None" "KeepWorld" "KeepRelative" "KeepRelative" true))))

(fn `Being Attacked Protected`
  (`PrimitiveComponent.SetCollisionResponseToChannel` (`self.CapsuleComponent`) "ECC_Pawn" "ECR_Overlap"))

(fn `CaculateEXPForLevelUp`
  (set `self.Levael_EXP` (* (`self.BaseEXP`) (`KismetMathLibrary.MultiplyMultiply_FloatFloat` (`self.Level UPCoe`) (`KismetMathLibrary.Conv_IntToDouble` (- (`self.Level`) 1))))))

(fn `EXP_Up`
  (params (EXP_Num :type "Float (double-precision)"))
  (locals (OverFlowEXP :type "Float (double-precision)"))
  (bind _output_get (set `self.Current_EXP` (+ (`self.Current_EXP`) EXP_Num)))
  (if (>= _output_get (`self.Levael_EXP`))
    (set `local.OverFlowEXP` (- (`self.Current_EXP`) (`self.Levael_EXP`)))
    (`/Engine/EditorBlueprintResources/StandardMacros.IncrementInt` (`self.Level`)
      (:`  `
        (`self.CaculateEXPForLevelUp`)
        (set `self.Current_EXP` 0.0)
        (`self.EXP_Up` (`local.OverFlowEXP`))
        (`/Game/UI/UI_PlayerMainUI.ShowSkillUP` (`self.MainUI`))))
    (else
      (`self.UpdateEXPHUD`))))

(fn `HUDInit`
  (bind _returnvalue (`|CreateWidget` "/Game/UI/UI_PlayerMainUI.UI_PlayerMainUI_C"))
  (bind _output_get (set `self.MainUI` _returnvalue))
  (`UserWidget.AddToViewport` _output_get 0)
  (`self.UpdateHPHUD`)
  (`self.UpdateEXPHUD`))

(fn `LearningSkill`
  (params (SkillTag :type String))
  (bind (_value _returnvalue) (`BlueprintMapLibrary.Map_Find` (`self.Skill Tag`) SkillTag))
  (if _returnvalue
    (bind _result (`/Engine/EditorBlueprintResources/StandardMacros.IncrementInt` _value)
      (:`  `
        (`BlueprintMapLibrary.Map_Add` (`self.Skill Tag`) (`local.SkillTag`) _result)
        (for (_array_element _array_index) (`self.SkillStruct`)
          (bind (_skilltag _skill_name _description _skilllevel _skillmaxlevel) (break `/Game/DataAsset/Skills/BP_Struct_Skills` _array_element))
          (if (`KismetStringLibrary.EqualEqual_StrStr` _skilltag (`local.SkillTag`))
            (if (== _result _skillmaxlevel)
              (`KismetArrayLibrary.Array_Remove` (`self.SkillStruct`) _array_index)
              (break))))))
    (else
      (`BlueprintMapLibrary.Map_Add` (`self.Skill Tag`) (`local.SkillTag`) 1)))
  (`/Game/UI/UI_PlayerMainUI.ShowSkillIcon` (`self.MainUI`))
  (`self.PassiveSkillUpgrade` (`local.SkillTag`))
  (`self.PositiveSkillUpgrade` (`local.SkillTag`)))

(fn `PassiveSkillUpgrade`
  (params (Skill :type String))
  (switch `string` Skill
    (:`DamageUP`
      (set `self.Damage` (+ (`self.Damage`) 5.0)))
    (:`HealthUP`
      (bind _output_get (set `self.Max Hp` (+ (`self.Max Hp`) 10.0)))
      (set `self.CurrentHP` _output_get)
      (`self.UpdateHPHUD`))
    (:`SpeedUP`
      (set `self.Speed` (+ (`self.Speed`) 10.0))
      (set `CharacterMovementComponent.MaxWalkSpeed` (`self.Speed`) (`self.CharacterMovement`)))
    (:`PickScaleUP`
      (set `self.PlayerPickScale` (+ (`self.PlayerPickScale`) 5.0))
      (`SphereComponent.SetSphereRadius` (`self.PickScale`) (`self.PlayerPickScale`) true))))

(fn `PlayerDAInit`
  (bind (_level _maxhp _damage _speed _pickscale _exp _startskilltag _levelupcoe) (`/Game/DataAsset/Player/DA_Player.GetPlayerDA` (`self.PlayerDA`)))
  (set `self.Level` _level)
  (set `self.Max Hp` _maxhp)
  (set `self.Damage` _damage)
  (set `self.Speed` _speed)
  (set `self.PlayerPickScale` _pickscale)
  (set `self.Start Skill Tag` _startskilltag)
  (set `CharacterMovementComponent.MaxWalkSpeed` (`self.Speed`) (`self.CharacterMovement`))
  (`SphereComponent.SetSphereRadius` (`self.PickScale`) (`self.PlayerPickScale`) true)
  (set `self.CurrentHP` (`self.Max Hp`))
  (set `self.BaseEXP` _exp)
  (set `self.Level UPCoe` _levelupcoe)
  (`self.CaculateEXPForLevelUp`)
  (`BlueprintMapLibrary.Map_Add` (`self.Skill Tag`) (`self.Start Skill Tag`) 1)
  (bind _outrownames (`DataTableFunctionLibrary.GetDataTableRowNames` "/Game/DataAsset/Skills/DT_SkillTable.DT_SkillTable"))
  (for _array_element _outrownames
    (bind _returnvalue (`|GetDataTableRow` "/Game/DataAsset/Skills/DT_SkillTable.DT_SkillTable" _array_element)
      (:`then`
        (`KismetArrayLibrary.Array_Add` (`self.SkillStruct`) _returnvalue)))))

(fn `PlayerHPCaculate`
  (params (Damage :type "Float (double-precision)"))
  (set `self.CurrentHP` (`KismetMathLibrary.FClamp` (- (`self.CurrentHP`) Damage) 0.0 (`self.Max Hp`)))
  (`self.UpdateHPHUD`)
  (if (<= (`self.CurrentHP`) 0.0)
    (set `self.isDeath` true)
    (`GameplayStatics.SetGamePaused` true)
    (bind _returnvalue (`|CreateWidget` "/Game/UI/UI_GameOver.UI_GameOver_C"))
    (bind _output_get (set `self.UIGameOver` _returnvalue))
    (`UserWidget.AddToViewport` _output_get 0)
    (`GameplayStatics.PlaySound2D` "/Game/Sound/SoundEffect/GameOver_Cue.GameOver_Cue" 1.0 1.0 0.0 null null)
    (else
      (`KismetSystemLibrary.K2_SetTimer` null "Being Attacked Protected" 0.2)
      (`PrimitiveComponent.SetCollisionResponseToChannel` (`self.CapsuleComponent`) "ECC_Pawn" "ECR_Overlap"))))

(fn `PositiveSkillUpgrade`
  (params (SkillTag :type String))
  (switch `string` SkillTag
    (:`Shuriken`
      (if (== (`self.ShurikenGainEffect`) 0.0)
        (bind _returnvalue (`|GetDataTableRow` "/Game/DataAsset/Skills/DT_SkillTable.DT_SkillTable" "Shuriken")
          (:`then`
            (set `self.ShurikenGainEffect` (`.GainEffect_21_C453812241BC5155B61733AF2CF35645` (break `/Game/DataAsset/Skills/BP_Struct_Skills` _returnvalue))))))
      (switch `int` (`BlueprintMapLibrary.Map_Find` (`self.Skill Tag`) "Shuriken")
        (:`2`
          (set `self.ShurikenSpeed` 200)
          (set `self.ShurikenNum` 2))
        (:`3`
          (set `self.ShurikenGainEffect` (+ (`self.ShurikenGainEffect`) 2.0)))
        (:`4`
          (set `self.ShurikenNum` 3)
          (set `self.Bullet Size` (1.23 1.23 1.23)))
        (:`5`
          (set `self.ShurikenLifeCycle` 2.0)
          (set `self.Bullet Size` (1.5 1.5 1.5))
          (set `self.ShurikenColor` (struct :`R` 1.0 :`A` 1.0))
          (set `self.ShurikenGainEffect` (* (`self.ShurikenGainEffect`) 1.5)))))
    (:`Thunder`
      (if (== (`self.ThunderGainEffect`) 0.0)
        (bind _returnvalue_2 (`|GetDataTableRow` "/Game/DataAsset/Skills/DT_SkillTable.DT_SkillTable" "Thunder")
          (:`then`
            (bind (_skilltag _skill_name _description _skilllevel _skillmaxlevel _rate _icon _gaineffect) (break `/Game/DataAsset/Skills/BP_Struct_Skills` _returnvalue_2))
            (set `self.ThunderGainEffect` _gaineffect)
            (set `self.ThunderRate` _rate)
            (`self.AutoAttack` "Thunder"))))
      (switch `int` (`BlueprintMapLibrary.Map_Find` (`self.Skill Tag`) "Thunder")
        (:`2`
          (set `self.ThunderTargetSize` (1.5 1.5 1.5))
          (set `self.ThunderGainEffect` (* (`self.ThunderGainEffect`) 1.1)))
        (:`3`
          (set `self.ThunderNum` 2)
          (set `self.ThunderRate` (* (`self.ThunderRate`) 0.8)))
        (:`4`
          (set `self.ThunderTargetSize` (2.0 2.0 2.0))
          (set `self.ThunderGainEffect` (* (`self.ThunderGainEffect`) 1.3)))
        (:`5`
          (set `self.ThunderNum` 3)
          (set `self.ThunderRate` (* (`self.ThunderRate`) 0.5))
          (set `self.ThunderTargetSize` (3.0 3.0 3.0))
          (set `self.ThunderColor` (struct :`R` 0.130764 :`G` 0.021055 :`B` 0.383333 :`A` 1.0))
          (set `self.ThunderSize` (1.0 1.0 1.0)))))
    (:`IceSword`
      (if (== (`self.IcrSwordGainEffect`) 0.0)
        (bind _returnvalue_3 (`|GetDataTableRow` "/Game/DataAsset/Skills/DT_SkillTable.DT_SkillTable" "IceSword")
          (:`then`
            (set `self.IcrSwordGainEffect` (`.GainEffect_21_C453812241BC5155B61733AF2CF35645` (break `/Game/DataAsset/Skills/BP_Struct_Skills` _returnvalue_3)))
            (`self.AutoAttack` "IceSword"))))
      (switch `int` (`BlueprintMapLibrary.Map_Find` (`self.Skill Tag`) "IceSword")
        (:`1`
          (set `self.ISRotattionRate` (struct :`Yaw` 60.0))
          (set `self.ISR` 35.0)
          (set `self.ISColor` (struct :`R` 1.0 :`G` 1.0 :`B` 1.0 :`A` 1.0))
          (set `self.ISBullet Size` (1.0 1.0 1.0))
          (set `self.ISItem Num` 1))
        (:`2`
          (set `self.ISRotattionRate` (struct :`Yaw` 90.0))
          (set `self.ISItem Num` 2))
        (:`3`
          (set `self.IcrSwordGainEffect` (* (`self.IcrSwordGainEffect`) 1.25))
          (set `self.ISBullet Size` (1.2 1.2 1.2)))
        (:`4`
          (set `self.ISRotattionRate` (struct :`Yaw` 120.0))
          (set `self.ISItem Num` 3))
        (:`5`
          (set `self.ISRotattionRate` (struct :`Yaw` 150.0))
          (set `self.ISItem Num` 5)
          (set `self.IcrSwordGainEffect` (* (`self.IcrSwordGainEffect`) 1.5))
          (set `self.ISBullet Size` (1.7 1.7 1.7))
          (set `self.ISColor` (struct :`R` 0.15882 :`B` 0.35 :`A` 1.0))))
      (bind _rotation (`self.Rotation`)
        (:`then`
          (`/Game/Bullet/BP_Rotation.setValue` _rotation (`self.ISRotattionRate`) (`self.ISR`) (`self.ISItem Num`) "/Game/Bullet/IceSword/IceSpike_Ani.IceSpike_Ani" (`self.IcrSwordGainEffect`) (`self.ISBullet Size`) 15.0 (`self.ISColor`))
          (`/Game/Bullet/BP_Rotation.BeginToRotation` _rotation))
        (:`else`)))))

(fn `RemoveMaxSkill`
  (params (SkillToRemove :type "/Game/DataAsset/Skills/BP_Struct_Skills Structure"))
  (`KismetArrayLibrary.Array_RemoveItem` (`self.SkillStruct`) SkillToRemove))

(fn `Skill_Shuriken`
  (bind _returnvalue (`self.K2_GetActorLocation`))
  (bind _bullet_size (`self.Bullet Size`))
  (bind (_returnvalue_roll _returnvalue_pitch _returnvalue_yaw) (`KismetMathLibrary.BreakRotator` (`KismetMathLibrary.FindLookAtRotation` _returnvalue (`.Location` (`GameplayStatics.BreakHitResult` (`PlayerController.GetHitResultUnderCursorByChannel` (`GameplayStatics.GetPlayerController` 0) "TraceTypeQuery1" true))))))
  (for _index (range (`self.ShurikenNum`))
    (bind _returnvalue_2 (select `int` _index :`0` -30.0 :`1` 30.0 :`2` 0.0))
    (`/Game/BluePrints/BP_ObjectPooling.setBulletPooling` (`/Game/BluePrints/Instance/GI_Instance_Bullet.ObjectPooling` (`self.As GI Instance Bullet`)) _returnvalue "/Game/Bullet/Shuriken/Shuriken_Attack.Shuriken_Attack" (+ (`self.Damage`) (`self.ShurikenGainEffect`)) (* (`KismetMathLibrary.Conv_RotatorToVector` (`KismetMathLibrary.MakeRotator` 0.0 0.0 (+ _returnvalue_yaw (select `int` (`self.ShurikenNum`) :`0` 0.0 :`1` 0.0 :`2` _returnvalue_2 :`3` _returnvalue_2)))) (`self.ShurikenSpeed`)) _bullet_size _bullet_size "enemy" (`self.ShurikenLifeCycle`) 10.0 (`self.ShurikenColor`))))

(fn `Skill_Thunder`
  (bind (_returnvalue_x _returnvalue_y _returnvalue_z) (`KismetMathLibrary.BreakVector` (`self.K2_GetActorLocation`)))
  (for _ (range (`self.ThunderNum`))
    (`/Game/BluePrints/BP_ObjectPooling.setBulletPooling` (`/Game/BluePrints/Instance/GI_Instance_Bullet.ObjectPooling` (`self.As GI Instance Bullet`)) (`KismetMathLibrary.MakeVector` (+ _returnvalue_x (`KismetMathLibrary.RandomFloatInRange` -50.0 50.0)) (+ _returnvalue_y (`KismetMathLibrary.RandomFloatInRange` -50.0 50.0)) _returnvalue_z) "/Game/Bullet/Thunder/Thunder_Ani.Thunder_Ani" (+ (`self.Damage`) (`self.ThunderGainEffect`)) (0.0 0.0 0.0) (`self.ThunderSize`) (`self.ThunderTargetSize`) "enemy" 0.5 10.0 (`self.ThunderColor`))))

(fn `UpdateEXPHUD`
  (`/Game/UI/UI_PlayerMainUI.UpdateEXP` (`self.MainUI`) (`self.Current_EXP`) (`self.Levael_EXP`))
  (`/Game/UI/UI_PlayerMainUI.UpdateLevel` (`self.MainUI`) (`self.Level`) (`self.Current_EXP`) (`self.Levael_EXP`)))

(fn `UpdateHPHUD`
  (`/Game/UI/UI_PlayerMainUI.UpdateHP` (`self.MainUI`) (`self.CurrentHP`) (`self.Max Hp`)))

(fn `UserConstructionScript`)