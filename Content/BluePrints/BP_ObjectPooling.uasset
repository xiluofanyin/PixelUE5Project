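; Object pool manager that registers itself on the GameInstance and supplies bullets, enemies and EXP items.
; Each setter reuses the first pooled actor in a given state, or spawns and stores a new one.
; It starts with ten enemies, and SetMoreEnemy tops up the active list below that target.
; A level clock updates the player's UI and determines the type of newly spawned enemies, alternating by parity after 20 seconds.
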(event `self.ReceiveBeginPlay`
  (set `/Game/BluePrints/Instance/GI_Instance_Bullet.ObjectPooling` self (`/Game/BluePrints/Instance/BL_PublicBPLibrary.GetGameInstance`))
  (`self.setEnemyNum` 10)
  (bind _returnvalue (`KismetSystemLibrary.K2_SetTimerDelegate` (`|CreateDelegate` :!event `LevelTime`) 1.0 true))
  (set `self.LeverTimer` _returnvalue))

(event `LevelTime`
  (bind _totaltime (`self.TotalTime`))
  (`/Engine/EditorBlueprintResources/StandardMacros.IncrementInt` _totaltime
    (:`  `
      (`/Game/UI/UI_PlayerMainUI.UpdateTime` (`/Game/BluePrints/BP_Player.MainUI` (`/Game/BluePrints/Instance/BL_PublicBPLibrary.GetPlayer`)) (/ _totaltime 60) (mod _totaltime 60)))))

(fn `setBulletPooling`
  (params (LaunchPosition :type "Vector Structure") (BulletPic :type "PaperFlipbook Object Reference") (BulletDamage :type "Float (double-precision)") (BulletSpeed :type "Vector Structure") (BulletSize :type "Vector Structure") (BulletTargetSize :type "Vector Structure") (BulletTarget :type Name) (LifeCycle :type "Float (double-precision)") (ImpactForce :type "Float (double-precision)") (Color :type "LinearColor Structure"))
  (locals (Bullet :type "/Game/Bullet/Shuriken/BP_Shuriken Object Reference"))
  (bind _bullet (`local.Bullet`))
  (for _array_element (`self.BulletPooling`)
    (if (`|EnumEquality` (`/Game/Bullet/Shuriken/BP_Shuriken.BulletState` _array_element) "NewEnumerator1")
      (set `local.Bullet` _array_element)
      (break)))
  (`local.Bullet`
    (:`then`
      _)
    (:`else`
      (bind _returnvalue (`|SpawnActorFromClass` "/Game/Bullet/Shuriken/BP_Shuriken.BP_Shuriken_C" (`KismetMathLibrary.MakeTransform` (10000.0 10000.0 -1000.0)) "Undefined" "OverrideRootScale" null null))
      (bind _output_get (set `local.Bullet` _returnvalue))
      (`KismetArrayLibrary.Array_Add` (`self.BulletPooling`) _output_get)))
  (`/Game/Bullet/Shuriken/BP_Shuriken.setBulletValue` _bullet (`local.BulletPic`) (`local.BulletDamage`) (`local.BulletSpeed`) (`local.BulletSize`) (`local.BulletTargetSize`) (`local.BulletTarget`) (`local.LifeCycle`) (`local.ImpactForce`) (`local.Color`))
  (`self.K2_SetActorLocation` _bullet (`local.LaunchPosition`) false false))

(fn `setEnemyNum`
  (params (EnemyNum :type Integer))
  (set `self.Enemy Num` EnemyNum)
  (for _ (range (`self.Enemy Num`))
    (`self.setEnemyPooling`)))

(fn `setEnemyPooling`
  (locals (Enemy :type "/Game/Enemies/BP_BaseEnemies Object Reference"))
  (for _array_element (`self.EnemyPooling`)
    (if (`|EnumEquality` (`/Game/Enemies/BP_BaseEnemies.EnemyState` _array_element) "NewEnumerator1")
      (set `local.Enemy` _array_element)
      (break)))
  (`local.Enemy`
    (:`then`
      _)
    (:`else`
      (if (> (`self.TotalTime`) 20)
        (if (== (mod (`self.TotalTime`) 2) 0)
          (set `self.Enemy Type` "NewEnumerator2" :!label _label)
          (else
            (set `self.Enemy Type` "NewEnumerator1")))
        (else
          (goto _label)))
      (bind _returnvalue (`|SpawnActorFromClass` "/Game/Enemies/BP_BaseEnemies.BP_BaseEnemies_C" (`KismetMathLibrary.MakeTransform` (0.0 0.0 -1000.0)) "Undefined" "OverrideRootScale" null (`self.Enemy Type`) null))
      (set `local.Enemy` _returnvalue)
      (`KismetArrayLibrary.Array_AddUnique` (`self.EnemyPooling`) (`local.Enemy`))))
  (set `/Game/Enemies/BP_BaseEnemies.EnemyState` "NewEnumerator0" (`local.Enemy`))
  (`KismetArrayLibrary.Array_Add` (`self.DynamicEnemyPooling`) (`local.Enemy`)))

(fn `setItemPooling`
  (params (EXP_Num :type "Float (double-precision)") (Position :type "Vector Structure"))
  (locals (Item :type "/Game/Item/BP_BaseItem Object Reference"))
  (for _array_element (`self.ItemPooling`)
    (if (`|EnumEquality` (`/Game/Item/BP_BaseItem.ItemState` _array_element) "NewEnumerator1")
      (set `local.Item` _array_element)
      (break)))
  (`local.Item`
    (:`then`
      _)
    (:`else`
      (bind _returnvalue (`|SpawnActorFromClass` "/Game/Item/BP_BaseItem.BP_BaseItem_C" (`KismetMathLibrary.MakeTransform` (200.0 200.0 -1000.0)) "Undefined" "OverrideRootScale" null null))
      (bind _output_get (set `local.Item` _returnvalue))
      (`KismetArrayLibrary.Array_AddUnique` (`self.ItemPooling`) _output_get)))
  (`/Game/Item/BP_BaseItem.setItemPooling` (`local.Item`) (`local.EXP_Num`))
  (`self.K2_SetActorLocation` (`local.Item`) (`local.Position`) false false))

(fn `setMoreEnemy`
  (if (< (`KismetArrayLibrary.Array_Length` (`self.DynamicEnemyPooling`)) (`self.Enemy Num`))
    (`self.setEnemyPooling`)))

(fn `UserConstructionScript`)