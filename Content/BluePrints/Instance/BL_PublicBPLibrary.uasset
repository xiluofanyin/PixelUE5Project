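; A Blueprint function library of shared static helpers for the game.
; GetGameInstance and GetPlayer return the game instance cast to GI_Instance_Bullet and player pawn 0 cast to BP_Player.
; CheckisInPlayerScreen projects a world location through player controller 0 and reports whether the screen point lies strictly inside the viewport bounds.
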(fn `CheckisInPlayerScreen`
  (params (WorldLocation :type "Vector Structure"))
  (returns (ReturnValue :type Boolean))
  (bind (_x _y) (`KismetMathLibrary.BreakVector2D` (`WidgetLayoutLibrary.GetViewportSize` null)))
  (bind (_x_2 _y_2) (`KismetMathLibrary.BreakVector2D` (`PlayerController.ProjectWorldLocationToScreen` (`GameplayStatics.GetPlayerController` null) WorldLocation false)))
  (return (and (> _x_2 0.0) (> _y_2 0.0) (< _x_2 _x) (< _y_2 _y))))

(fn `GetGameInstance`
  (returns (`AsGI Instance Bullet` :type "/Game/BluePrints/Instance/GI_Instance_Bullet Object Reference"))
  (bind _asgi_instance_bullet (cast `/Game/BluePrints/Instance/GI_Instance_Bullet` (`GameplayStatics.GetGameInstance` null)))
  (return _asgi_instance_bullet))

(fn `GetPlayer`
  (returns (`AsBP Player` :type "/Game/BluePrints/BP_Player Object Reference"))
  (bind _asbp_player (cast `/Game/BluePrints/BP_Player` (`GameplayStatics.GetPlayerPawn` null)))
  (return _asbp_player))