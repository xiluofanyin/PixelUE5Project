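; BP_BaseItem is a pooled 2D pickup, such as a coin, letter, octopus or kill-all, that flies to whatever overlaps its sphere.
; Its Type selects the flipbook at BeginPlay and the sound played on collection.
; Overlap starts a timeline that interpolates it toward the actor and, when close, calls GetPickItemMessage.
; It then recycles by changing ItemState and moving off-field instead of being destroyed, while SetItemPooling resets state and EXP.
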(event `self.ReceiveBeginPlay`
  (switch `/Game/BluePrints/Enum/Enum_ItemType` (`self.Type`)
    (:`NewEnumerator0`
      (set `self.PicSequence` "/Game/Item/Asset/Coin_Sequence.Coin_Sequence"))
    (:`NewEnumerator1`
      (set `self.PicSequence` "/Game/Item/Asset/Letter_Sequence.Letter_Sequence"))
    (:`NewEnumerator2`
      (set `self.PicSequence` "/Game/Item/Asset/Octopus_Sequence.Octopus_Sequence"))
    (:`NewEnumerator3`
      (set `self.PicSequence` "/Game/Item/Asset/KillAll.KillAll")))
  (`PaperFlipbookComponent.SetFlipbook` (`self.PaperFlipbook`) (`self.PicSequence`)))

(event `self.Sphere.OnComponentBeginOverlap`
  (params (OverlappedComponent :type "PrimitiveComponent Object Reference") (OtherActor :type "Actor Object Reference") (OtherComp :type "PrimitiveComponent Object Reference") (OtherBodyIndex :type Integer) (bFromSweep :type Boolean) (SweepResult :type "HitResult Structure (by ref)"))
  (set `self.Player` OtherActor)
  (`Timeline|时间轴` :!via `PlayFromStart`
    (:`Update`
      (`self.K2_SetActorLocation` (`KismetMathLibrary.VInterpTo` (`self.K2_GetActorLocation`) (`self.K2_GetActorLocation` (`self.Player`)) (`GameplayStatics.GetWorldDeltaSeconds`) 10.0))
      (if (<= (`self.GetDistanceTo` self (`self.Player`)) 5.0)
        (message `/Game/Interface/BP_Interface_Player.GetPickItem` (`self.Player`) self)
        (`TimelineComponent.Stop` (`self.时间轴`))
        (`self.ItemRecycling`)))))

(fn `ItemRecycling`
  (set `self.ItemState` "NewEnumerator1")
  (`self.K2_SetActorLocation` (200.0 200.0 -1000.0))
  (switch `/Game/BluePrints/Enum/Enum_ItemType` (`self.Type`)
    (:`NewEnumerator0`
      (set `self.Sound` "/Game/Sound/SoundEffect/Coin_Sound.Coin_Sound"))
    (:`NewEnumerator1`
      (set `self.Sound` null))
    (:`NewEnumerator2`
      (set `self.Sound` null))
    (:`NewEnumerator3`
      (set `self.Sound` "/Game/Sound/SoundEffect/Magic1_Cue.Magic1_Cue")))
  (bind _sound (`self.Sound`)
    (:`then`
      (`GameplayStatics.PlaySound2D` _sound 1.0 1.0 0.0 null null))
    (:`else`)))

(fn `setItemPooling`
  (params (EXP_Num :type "Float (double-precision)"))
  (set `self.EXP Num` EXP_Num)
  (set `self.ItemState` "NewEnumerator0"))

(fn `UserConstructionScript`)