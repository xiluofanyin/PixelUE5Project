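; BP_KillAll is a short-lived item actor that kills enemies inside a screen-sized area.
; On BeginPlay it sets its box extent from the viewport's pixel width and height with a fixed depth, then destroys itself after a brief delay.
; While it exists, any overlapping actor tagged "enemy" receives a BeingAttackedMessage with massive damage and no impact force.
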(event `self.ReceiveBeginPlay`
  (`self.setScale`)
  (`KismetSystemLibrary.Delay` 0.2)
  (`self.K2_DestroyActor`))

(event `self.Box.OnComponentBeginOverlap`
  (params (OverlappedComponent :type "PrimitiveComponent Object Reference") (OtherActor :type "Actor Object Reference") (OtherComp :type "PrimitiveComponent Object Reference") (OtherBodyIndex :type Integer) (bFromSweep :type Boolean) (SweepResult :type "HitResult Structure (by ref)"))
  (if (`self.ActorHasTag` OtherActor "enemy")
    (message `/Game/Interface/BP_Interface_Enemy.Being Attacked` OtherActor 9999.0 0.0)))

(fn `setScale`
  (bind (_returnvalue_x _returnvalue_y) (`KismetMathLibrary.BreakVector2D` (`WidgetLayoutLibrary.GetViewportSize`)))
  (`BoxComponent.SetBoxExtent` (`self.Box`) (`KismetMathLibrary.MakeVector` _returnvalue_x _returnvalue_y 32.0) true))

(fn `UserConstructionScript`)